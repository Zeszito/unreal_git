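; Zombie AI pawn that alternates at random between wandering the navmesh and chasing the player, starting with a wander on BeginPlay.
; AI MoveTo drives both states: a coin flip after each successful move picks the next, with a short pause after wandering.
; A failed chase returns to wandering, while a failed wander ends the loop.
; No attack logic exists, and the player-reference caching event is never called here.
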(event Custom|MoveToRandomLocation
  ;[1 1 1] Andar as voltas
  (AI|AIMoveTo self (.RandomLocation (Class|NavigationSystemV1|GetRandomPointinNavigableRadius (Transformation|GetActorLocation) 3e+02 0 0)) 0 5.0 false
    (:OnSuccess
      (Utilities|FlowControl|Delay 2.0)
      (if (Math|Random|RandomBool)
        (CallFunction|MovetoRandomLocation)
        (else
          (CallFunction|FollowPlayer))))))

(event Custom|FollowPlayer
  ;[1 1 1] Find player and atack or flee
  (AI|AIMoveTo self "0, 0, 0" (Game|GetPlayerCharacter 0) 5e+01 false
    (:OnSuccess
      (if (Math|Random|RandomBool)
        (CallFunction|MovetoRandomLocation)
        (else
          (CallFunction|FollowPlayer))))
    (:OnFail
      (CallFunction|MovetoRandomLocation))))

(event Custom|CustomEvent
  ;[1 1 1] Get player REf
  (bind _asthird_person_character (Utilities|Casting|CastToThirdPersonCharacter (Game|GetPlayerCharacter 0)))
  (Variables|Default|SetplayerRef _asthird_person_character))

(event EventBeginPlay
  (CallFunction|MovetoRandomLocation))

(fn ConstructionScript)