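; Zombie character Blueprint that moves toward the player while an overlap flag is set.
; Capsule overlap with a "Player"-tagged actor sets the flag, and any end overlap clears it.
; While set, Tick calls a timed MoveComponentTo on the capsule toward the cached player's XY at its own height.
; Target rotation comes from negating the combined forward vectors of zombie and player.
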(event OnComponentBeginOverlap(CapsuleComponent)
  (params (OverlappedComponent :type Primitive%20Component%20Object%20Reference) (OtherActor :type Actor%20Object%20Reference) (OtherComp :type Primitive%20Component%20Object%20Reference) (OtherBodyIndex :type Integer) (bFromSweep :type Boolean) (SweepResult :type Hit%20Result%20Structure%20%28by%20ref%29))
  ;[1 1 1] Player enter Colider
  (if (Actor|ActorHasTag OtherActor "Player")
    (Variables|Default|SetEntrou true)))

(event OnComponentEndOverlap(CapsuleComponent)
  (params (OverlappedComponent :type Primitive%20Component%20Object%20Reference) (OtherActor :type Actor%20Object%20Reference) (OtherComp :type Primitive%20Component%20Object%20Reference) (OtherBodyIndex :type Integer))
  (Variables|Default|Setentrou false))

(event EventBeginPlay
  ;[1 1 1] Get player REf
  (bind _asthird_person_character (Utilities|Casting|CastToThirdPersonCharacter (Game|GetPlayerCharacter 0)))
  (Variables|Default|SetplayerREf _asthird_person_character))

(event Collision|EventActorBeginOverlap
  (params (OtherActor :type Actor%20Object%20Reference)))

(event EventTick
  (params (DeltaSeconds :type Float%20%28single-precision%29))
  (bind _playerref (Variables|Default|GetplayerREf))
  (bind _capsulecomponent (Variables|Collision|GetCapsuleComponent))
  (bind _returnvalue (Transformation|GetActorLocation _playerref))
  (if (Variables|Default|GetEntrou)
    ;[1 1 1] Logica de movimento
    (Components|MoveComponentTo _capsulecomponent (Math|Vector|MakeVector (.x _returnvalue) (.y _returnvalue) (.z (Transformation|GetWorldLocation _capsulecomponent))) (Math|Conversions|RotationFromXVector (* (Math|Rotator|GetRotationXVector (Math|Conversions|RotationFromXVector (+ (Math|Rotator|GetRotationXVector (Transformation|GetActorRotation self)) (Math|Rotator|GetRotationXVector (Transformation|GetActorRotation _playerref))))) -1)) false false 5.0 false)))

(fn ConstructionScript)