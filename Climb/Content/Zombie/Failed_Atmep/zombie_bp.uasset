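; Zombie Blueprint that follows the player while they overlap its capsule and returns to its spawn transform otherwise.
; BeginPlay caches the player character and start transform; capsule overlaps set the Entrou flag, with the Player tag checked only on entry.
; Tick issues one-second MoveComponentTo calls toward the player's X/Y at the capsule's own height, rotated opposite the player's facing, or back to the start.
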(event OnComponentBeginOverlap(Capsule)
  (params (OverlappedComponent :type Primitive%20Component%20Object%20Reference) (OtherActor :type Actor%20Object%20Reference) (OtherComp :type Primitive%20Component%20Object%20Reference) (OtherBodyIndex :type Integer) (bFromSweep :type Boolean) (SweepResult :type Hit%20Result%20Structure%20%28by%20ref%29))
  (if (Actor|ActorHasTag OtherActor "Player")
    (Variables|Default|Setentrou true)))

(event OnComponentEndOverlap(Capsule)
  (params (OverlappedComponent :type Primitive%20Component%20Object%20Reference) (OtherActor :type Actor%20Object%20Reference) (OtherComp :type Primitive%20Component%20Object%20Reference) (OtherBodyIndex :type Integer))
  (Variables|Default|Setentrou false))

(event EventBeginPlay
  ;[1 1 1] Get char ref
  (bind _asthird_person_character (Utilities|Casting|CastToThirdPersonCharacter (Game|GetPlayerCharacter 0)))
  (Variables|Default|SetAs%20Third%20Person%20Character _asthird_person_character)
  (Variables|Default|Setoriginal%20pos (Transformation|GetWorldLocation (Variables|Default|GetCapsule)))
  (Variables|Default|Setorignal%20rot (Transformation|GetActorRotation self)))

(event Collision|EventActorBeginOverlap
  (params (OtherActor :type Actor%20Object%20Reference)))

(event EventTick
  (params (DeltaSeconds :type Float%20%28single-precision%29))
  (bind _capsule (Variables|Default|GetCapsule))
  (bind _as_third_person_character (Variables|Default|GetAs%20Third%20Person%20Character))
  (bind _original_pos (Variables|Default|Getoriginal%20pos))
  (bind _returnvalue (Transformation|GetActorLocation _as_third_person_character))
  (if (Variables|Default|Getentrou)
    (Components|MoveComponentTo _capsule (Math|Vector|MakeVector (.x _returnvalue) (.y _returnvalue) (.z (Transformation|GetWorldLocation _capsule))) (Math|Conversions|RotationFromXVector (* (Math|Vector|GetForwardVector (Math|Conversions|RotationFromXVector (Math|Rotator|GetRotationXVector (Transformation|GetActorRotation _as_third_person_character)))) -1)) false false 1.0 false)
    (else
      (Components|MoveComponentTo _capsule (Math|Vector|MakeVector (.x _original_pos) (.y _original_pos) (.z _original_pos)) (Variables|Default|Getorignal%20rot) false false 1.0 false))))

(fn ConstructionScript)