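; Zombie actor Blueprint that moves toward the player while a trigger box is occupied, apparently an abandoned attempt going by its folder.
; BeginPlay caches the player character; overlap by a "Player"-tagged actor sets a flag, and any end overlap clears it.
; While flagged, Tick calls a timed MoveComponentTo on the capsule toward the player's X/Y, keeping its height and rotating opposite the player's forward vector.
; The GoToPlayer event is empty.
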(event OnComponentBeginOverlap(box)
  (params (OverlappedComponent :type Primitive%20Component%20Object%20Reference) (OtherActor :type Actor%20Object%20Reference) (OtherComp :type Primitive%20Component%20Object%20Reference) (OtherBodyIndex :type Integer) (bFromSweep :type Boolean) (SweepResult :type Hit%20Result%20Structure%20%28by%20ref%29))
  ;[1 1 1] Player enter Colider
  (if (Actor|ActorHasTag OtherActor "Player")
    (Variables|Default|Setentrou true)))

(event OnComponentEndOverlap(box)
  (params (OverlappedComponent :type Primitive%20Component%20Object%20Reference) (OtherActor :type Actor%20Object%20Reference) (OtherComp :type Primitive%20Component%20Object%20Reference) (OtherBodyIndex :type Integer))
  (Variables|Default|Setentrou false))

(event Custom|GoToPlayer)

(event EventBeginPlay
  ;[1 1 1] Get player REf
  (bind _asthird_person_character (Utilities|Casting|CastToThirdPersonCharacter (Game|GetPlayerCharacter 0)))
  (Variables|Default|SetPlayerRef _asthird_person_character))

(event Collision|EventActorBeginOverlap
  (params (OtherActor :type Actor%20Object%20Reference)))

(event EventTick
  (params (DeltaSeconds :type Float%20%28single-precision%29))
  (bind _playerref (Variables|Default|GetPlayerRef))
  (bind _capsule (Variables|Default|GetCapsule))
  (bind _returnvalue (Transformation|GetActorLocation _playerref))
  (if (Variables|Default|Getentrou)
    ;[1 1 1] Logica de movimento
    (Components|MoveComponentTo _capsule (Math|Vector|MakeVector (.x _returnvalue) (.y _returnvalue) (.z (Transformation|GetWorldLocation _capsule))) (Math|Conversions|RotationFromXVector (* (Math|Vector|GetForwardVector (Transformation|GetActorRotation _playerref)) -1)) false false 1e+01 false)))

(fn ConstructionScript)