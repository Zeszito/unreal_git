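; Door actor that opens once when a player carrying a key overlaps its Box trigger.
; BeginPlay caches the ThirdPersonCharacter reference; the overlap checks the Player tag, that character's HasKey and the DoorMoved flag.
; DoorOpens instantly shifts the door mesh along Z by an offset scaled from its world Z, so travel depends on placement.
; Opening clears the player's key and sets DoorMoved to block repeats.
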(event OnComponentBeginOverlap(Box)
  (params (OverlappedComponent :type Primitive%20Component%20Object%20Reference) (OtherActor :type Actor%20Object%20Reference) (OtherComp :type Primitive%20Component%20Object%20Reference) (OtherBodyIndex :type Integer) (bFromSweep :type Boolean) (SweepResult :type Hit%20Result%20Structure%20%28by%20ref%29))
  ;[1 1 1] Detecta player com chave
  (if (and (and (Actor|ActorHasTag OtherActor "Player") (Variables|/Game/ThirdPersonBP/Blueprints/ThirdPersonCharacter.ThirdPersonCharacter_C|GethasKey (Variables|Default|GetplayerREf))) (not (Variables|Default|GetdoorMoved)))
    (CallFunction|DoorOpens)
    (Variables|/Game/ThirdPersonBP/Blueprints/ThirdPersonCharacter.ThirdPersonCharacter_C|SethasKey (Variables|Default|GetplayerREf) false)
    (Variables|Default|SetdoorMoved true)))

(event Custom|DoorOpens
  (bind _porta1ue4_porta (Variables|Default|Getporta1UE4_Porta))
  (bind _returnvalue (Transformation|GetWorldLocation _porta1ue4_porta))
  (Transformation|SetWorldLocation _porta1ue4_porta (Math|Vector|MakeVector (.x _returnvalue) (.y _returnvalue) (- (.z _returnvalue) (* (.z _returnvalue) 4.0))) false false))

(event EventBeginPlay
  ;[1 1 1] Get player REf
  (bind _asthird_person_character (Utilities|Casting|CastToThirdPersonCharacter (Game|GetPlayerCharacter 0)))
  (Variables|Default|SetplayerREf _asthird_person_character)
  ;[1 1 1] door moved? NOT
  (Variables|Default|SetdoorMoved false))

(event Collision|EventActorBeginOverlap
  (params (OtherActor :type Actor%20Object%20Reference)))

(fn ConstructionScript)